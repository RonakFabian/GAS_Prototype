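; Enemy actor that turns to face the player and plays a punch-to-the-face reaction montage when its Damage event fires.
; Tick passes the player pawn to LookAt, which runs a timeline that lerps actor rotation along the shortest path toward the target.
; Only yaw targets the player; roll and pitch come from the mesh's world rotation, which is also the lerp's starting point.
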(event Custom|LookAt
  (params (Target :type Actor%20Object%20Reference))
  (bind _mesh (Variables|Character|GetMesh))
  (bind _returnvalue (Transformation|GetWorldRotation _mesh))
  (bind (_roll _pitch) (Math|Rotator|BreakRotator _returnvalue))
  ;[1 1 1] Comment
  (bind _alpha (Timeline|Timeline_2 Play)
    (:Update
      (Transformation|SetActorRotation (Math|Rotator|Lerp(Rotator) _returnvalue (Math|Rotator|MakeRotator _roll _pitch (.yaw (Math|Rotator|FindLookatRotation (Transformation|GetWorldLocation (Variables|Character|GetMesh)) (Transformation|GetWorldLocation (Variables|/Script/Engine.Actor|GetRootComponent Target))))) _alpha true) true))))

(event EventBeginPlay
  (|CallParentFunction) ; This node is disabled and will not be called.\nDrag off pins to build functionality.
)

(event Collision|EventActorBeginOverlap
  (params (OtherActor :type Actor%20Object%20Reference)))

(event EventTick
  (params (DeltaSeconds :type Float%20%28single-precision%29))
  (|CallParentFunction DeltaSeconds)
  (CallFunction|Lookat (Game|Player|GetPlayerPawn 0)))

(event EventDamage
  (Animation|Montage|PlayMontage (Variables|Character|GetMesh) "/Game/Anims/AM_ReceivePunchToTheFace4UE4_Montage.AM_ReceivePunchToTheFace4UE4_Montage"))

(fn ConstructionScript
  (|CallParentFunction))
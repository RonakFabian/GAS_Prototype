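; Enemy manager that randomly gives each enemy in its Enemies array one of two role numbers at game start.
; On BeginPlay it fills a Roles array with random rolls, copies them by index to each enemy's RoleNumber, then prints the results.
; GetRandomEnemy returns a random entry from the array, and AssignEnemyState is an empty event.
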(event Custom|Assign%20Enemy%20State)

(event EventBeginPlay
  (for _index (range 0 (Utilities|Array|Length (Variables|Default|GetEnemies)))
    (Utilities|Array|Add (Variables|Default|GetRoles) (Math|Random|RandomIntegerinRange 1 2)))
  (for (_array_element _array_index) (Variables|Default|GetEnemies)
    (Variables|/Game/BP_Enemy.BP_Enemy_C|SetRoleNumber _array_element (Utilities|Array|Get(acopy) (Variables|Default|GetRoles) _array_index)))
  (for _array_element_2 (Variables|Default|GetEnemies)
    (Development|PrintString (Utilities|String|ToString(Integer) (Variables|/Game/BP_Enemy.BP_Enemy_C|GetRoleNumber _array_element_2)))))

(fn ConstructionScript)

(fn GetRandomEnemy
  (return (.OutItem (Utilities|Array|Random (Variables|Default|GetEnemies)))))